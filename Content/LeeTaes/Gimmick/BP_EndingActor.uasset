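; BP_EndingActor is a gimmick actor that runs the game's ending and then returns to the lobby level.
; StartEnding plays the stored level sequence, hides player 0's character mesh in game, and binds a custom event to the sequence player's finish.
; That event opens LobbyLevel by object reference, while TestFunc assigns the sequence to play.
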(event Custom|커스텀이벤트
  (Game|OpenLevel(byObjectReference) "/Game/sangun/Lobby/LobbyLevel.LobbyLevel"))

(event EventStartEnding
  (bind _sequence (Variables|Default|GetSequence))
  (bind _sequenceplayer (Variables|/Script/LevelSequence.LevelSequenceActor|GetSequencePlayer _sequence))
  (Sequencer|Player|Play _sequenceplayer :!class /Script/MovieScene.MovieSceneSequencePlayer)
  (Development|SetHiddeninGame (Variables|/Script/Engine.Character|GetMesh (Game|GetPlayerCharacter 0)) true false)
  (EventDispatchers|BindEventtoOnFinished _sequenceplayer (delegate Custom|커스텀이벤트)))

(event Collision|EventActorBeginOverlap
  (params (OtherActor :type Actor%20Object%20Reference)))

(event EventTick
  (params (DeltaSeconds :type Float%20%28single-precision%29)))

(fn ConstructionScript)

(fn TestFunc
  (params (NewParam :type Level%20Sequence%20Actor%20Object%20Reference))
  (Variables|Default|SetSequence NewParam))