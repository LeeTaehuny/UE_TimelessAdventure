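; BP_InventoryComponent is an inventory component that holds the item array and owns the inventory UI.
; On BeginPlay it creates a WBP_Inventory widget, resizes Items to twelve slots and passes itself to the widget's LoadInventory.
; The B key toggles the widget on screen, using its visibility to choose between removing it from its parent and adding it to the viewport.
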(event EventBeginPlay
  (bind _returnvalue (UserInterface|CreateWidget "/Game/ykyung/Inventory/WBP_Inventory.WBP_Inventory_C"))
  (Variables|Default|SetInventoryWidget _returnvalue)
  (Utilities|Array|Resize (Variables|Default|GetItems) 12)
  (Default|LoadInventory (Variables|Default|GetInventoryWidget) self))

(event EventTick
  (params (DeltaSeconds :type Float%20%28single-precision%29)))

(event Input|KeyboardEvents|B
  (params (Key :type Key%20Structure :default "None"))
  (bind _inventorywidget (Variables|Default|GetInventoryWidget))
  (:Pressed
    (if (Widget|IsVisible (Variables|Default|GetInventoryWidget))
      (Widget|RemovefromParent _inventorywidget)
      (else
        (UserInterface|Viewport|AddtoViewport _inventorywidget 0)))))