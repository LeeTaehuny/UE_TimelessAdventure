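; BP_Patrol is a patrol route actor that supplies waypoints for enemy AI along a spline.
; GetSplinePoint returns the world location of the spline point at the current PatrolIndex.
; IncrementPatrol steps that index by PatrolDirection and flips the direction at the first and last points, so the route is walked back and forth rather than looped.
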(event Custom|IncrementPatrol
  (bind _output_get (Variables|Default|SetPatrolIndex (+ (Variables|Default|GetPatrolIndex) (Variables|Default|GetPatrolDirection))))
  (if (== _output_get (- (Spline|GetNumberOfSplinePoints (Variables|Default|GetPatrolSpline)) 1))
    (Variables|Default|SetPatrolDirection -1)
    (elif (== (Variables|Default|GetPatrolIndex) 0)
      (Variables|Default|SetPatrolDirection 1))))

(fn ConstructionScript)

(fn GetSplinePoint
  (return (Spline|GetLocationatSplinePoint (Variables|Default|GetPatrolSpline) (Variables|Default|GetPatrolIndex) "World")))